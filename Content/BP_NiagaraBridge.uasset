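; Bridge actor intended to pass Niagara particle positions to the MetaAgent player controller.
; On BeginPlay it sets the Niagara component's User.ParticleCallbackHandler to the component itself, not the actor, then activates it.
; An unconnected ReceiveParticleData chain would collect particle positions, submit them through SubmitNiagaraParticlePositions and print a debug message.
; That chain never runs, so no data reaches the controller.
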(event EventBeginPlay
  (Class|NiagaraComponent|SetVariableObject (Variables|Default|GetNIAGARAFX) "User.ParticleCallbackHandler" (Variables|Default|GetNIAGARAFX))
  (Components|Activation|Activate (Variables|Default|GetNIAGARAFX) false))

(event Collision|EventActorBeginOverlap
  (params (OtherActor :type Actor%20Object%20Reference)))

(event EventTick
  (params (DeltaSeconds :type Float%20%28single-precision%29)))

(fn ConstructionScript)